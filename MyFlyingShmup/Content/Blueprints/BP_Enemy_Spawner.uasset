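; Enemy spawner that continuously spawns random enemy classes from EnemyClassPool, starting at BeginPlay.
; A self-requeuing timer, currently fixed at one second, triggers each spawn and schedules the next.
; Each enemy spawns at a random point along the StartLocation spline, rotated to face a random point along the EndLocation spline.
; Class, position and delay draws share one random stream, reset on BeginPlay for repeatable sequences.
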(event Custom|SpawnEnemy
  (bind (_startlocation _endlocation) (CallFunction|GetStartandEndLocation))
  (Game|SpawnActorfromClass (.OutItem (Utilities|Array|RandomFromStream (Variables|Default|GetEnemyClassPool) (Variables|Default|GetRandonStream))) (Math|Transform|MakeTransform _startlocation (Math|Rotator|FindLookatRotation _startlocation _endlocation) "1.000000,1.000000,1.000000") "Undefined" "MultiplyWithRoot" 0 0)
  (CallFunction|QueueEnemySpawn))

(event Custom|QueueEnemySpawn
  (bind _returnvalue (Utilities|Time|SetTimerbyEvent (delegate Custom|SpawnEnemy) (Math|Random|RandomFloatinRangefromStream (Variables|Default|GetRandonStream) 1.0 1.0) false true))
  (Variables|Default|SetEnemySpawnTimer _returnvalue))

(event EventBeginPlay
  (Class|KismetMathLibrary|ResetRandomStream (Variables|Default|GetRandonStream))
  (CallFunction|QueueEnemySpawn))

(fn ConstructionScript)

(fn GetStartandEndLocation
  (return (Spline|GetLocationatTime (Variables|Default|GetStartLocation) (Math|Random|RandomFloatfromStream (Variables|Default|GetRandonStream)) "World" false) (Spline|GetLocationatTime (Variables|Default|GetEndLocation) (Math|Random|RandomFloatfromStream (Variables|Default|GetRandonStream)) "World" false)))