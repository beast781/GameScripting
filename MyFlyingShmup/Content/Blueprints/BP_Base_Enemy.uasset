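; BP_Base_Enemy is a base enemy actor that takes damage from projectiles and is destroyed when its health runs out.
; On overlap with a BP_Projectile, it passes the projectile's damage to ApplyDamage, which subtracts it from Health.
; A lethal hit plays an explosion sound and destroys the actor.
; Other hits play a laser sound and briefly flash every static mesh component using a damage overlay material.
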(event Custom|ApplyDamage
  (params (Damage :type Float%20%28double-precision%29))
  (Variables|Default|SetHealth (- (Variables|Default|GetHealth) Damage)))

(event Collision|EventActorBeginOverlap
  (params (OtherActor :type Actor%20Object%20Reference))
  (bind _asbp_projectile (Utilities|Casting|CastToBP_Projectile OtherActor))
  (CallFunction|ApplyDamage (Variables|/Game/Blueprints/BP_Projectile.BP_Projectile_C|GetDamage _asbp_projectile))
  (if (<= (Variables|Default|GetHealth) 0.0)
    (Audio|PlaySound2D "/Game/Audio/Explosion.Explosion" 0.1 1.0 0.0 0 0)
    (Actor|DestroyActor)
    (else
      (Audio|PlaySound2D "/Game/Audio/laser-312360.laser-312360" 0.1 1.0 0.0 0 0)
      (for _array_element (Actor|GetComponentsByClass "/Script/Engine.StaticMeshComponent")
        (Rendering|Material|SetOverlayMaterial _array_element "/Game/Materials/MI_Damage_Flash.MI_Damage_Flash" :!class /Script/Engine.MeshComponent))
      (Utilities|FlowControl|Delay 0.2)
      (for _array_element_2 (Actor|GetComponentsByClass "/Script/Engine.StaticMeshComponent")
        (Rendering|Material|SetOverlayMaterial _array_element_2 0 :!class /Script/Engine.MeshComponent))
      (Utilities|FlowControl|Delay 0.2))))

(fn ConstructionScript)