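; BP_Enemy_Turret is an enemy turret that tracks the player and fires lasers on a fixed interval.
; Each tick it rotates TurretBase in yaw only toward the first player's pawn.
; A looping timer started at BeginPlay spawns a BP_Enemy_Laser at the BulletSpawnPoint transform, with no range or line-of-sight check.
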(event Custom|ShootBullet
  (Game|SpawnActorfromClass "/Game/Blueprints/BP_Enemy_Laser.BP_Enemy_Laser_C" (Transformation|GetWorldTransform (Variables|Default|GetBulletSpawnPoint)) "AlwaysSpawn" "MultiplyWithRoot" 0 0))

(event EventBeginPlay
  (|CallParentFunction)
  (Utilities|Time|SetTimerbyEvent (delegate Custom|ShootBullet) 3.0 true true))

(event EventTick
  (params (DeltaSeconds :type Float%20%28single-precision%29))
  (Transformation|SetWorldRotation (Variables|Default|GetTurretBase) (Math|Rotator|MakeRotator 0.0 0.0 (.yaw (Math|Rotator|FindLookatRotation (Transformation|GetActorLocation) (Transformation|GetActorLocation (Game|Player|GetPlayerPawn 0))))) false false))

(fn ConstructionScript
  (|CallParentFunction))