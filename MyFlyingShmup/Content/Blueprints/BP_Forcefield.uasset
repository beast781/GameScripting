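; BP_Forcefield is a destructible forcefield actor that damages actors overlapping it.
; On overlap it waits one tick, then deals damage equal to its current Life, so a weakened field hits for less.
; Incoming damage reduces the clamped Life value, prints it on screen, and destroys the actor when it reaches zero.
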(event Collision|EventActorBeginOverlap
  (params (OtherActor :type Actor%20Object%20Reference))
  (Utilities|FlowControl|DelayUntilNextTick)
  (Game|Damage|ApplyDamage OtherActor (Variables|Default|GetLife) 0 0))

(event Game|Damage|EventAnyDamage
  (params (Damage :type Float%20%28single-precision%29) (DamageType :type Damage%20Type%20Object%20Reference) (InstigatedBy :type Controller%20Object%20Reference) (DamageCauser :type Actor%20Object%20Reference))
  (bind _output_get (Variables|Default|SetLife (Math|Float|Clamp(Float) (- (Variables|Default|GetLife) Damage) 0.0 3e+02)))
  (Development|PrintString (Utilities|String|ToString(Float) (Variables|Default|GetLife)))
  (if (== _output_get 0.0)
    (Actor|DestroyActor)))

(fn ConstructionScript)